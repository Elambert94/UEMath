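; Procedural quad actor with an arrow, apparently a visual aid for surface normals in a cross-product demo, though it computes no normals itself.
; UpdateMesh builds a four-vertex square of a given length with CreateGridMeshTriangles, then centers the arrow on the mesh bounds and scales its length.
; Separate functions set the plane's world rotation one axis at a time and the arrow's rotation, with BeginPlay and construction left empty.
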(event `self.ReceiveBeginPlay`)

(fn `DrawQuad`
  (params (Length :type "Float (double-precision)"))
  (returns (VertexArr :type "Array of Vector Structure"))
  (locals (X :type Integer) (Y :type Integer) (Vertex :type "Array of Vector Structure"))
  (bind _length (`local.Length`))
  (for _index (range 2)
    (set `local.X` _index)
    (for _index_2 (range 2)
      (set `local.Y` _index_2)
      (`KismetArrayLibrary.Array_Add` (`local.Vertex`) (`KismetMathLibrary.MakeVector` (* (`local.X`) _length) (* (`local.Y`) _length)))))
  (return (`local.Vertex`)))

(fn `GenerateMesh`
  (params (VertexArr :type "Array of Vector Structure"))
  (bind _triangles (`KismetProceduralMeshLibrary.CreateGridMeshTriangles` 2 2))
  (`ProceduralMeshComponent.CreateMeshSection_LinearColor` :`self` (`self.ProceduralMesh`) :`Vertices` (`local.VertexArr`) :`Triangles` _triangles))

(fn `SetArrowAngle`
  (params (NewRotation :type "Rotator Structure"))
  (`SceneComponent.K2_SetWorldRotation` (`self.Arrow`) NewRotation false false))

(fn `SetPlaneRotation`
  (params (InRot :type "Float (double-precision)") (Axis :type "EAxis Enum" :default "None"))
  (locals (Rot :type "Rotator Structure" :default (struct)))
  (bind _returnvalue (`SceneComponent.K2_GetComponentRotation` (`self.ProceduralMesh`)))
  (switch `EAxis` Axis
    (:`X`
      (set `local.Rot` (`KismetMathLibrary.MakeRotator` (`local.InRot`) (.pitch _returnvalue) (.yaw _returnvalue))))
    (:`Y`
      (set `local.Rot` (`KismetMathLibrary.MakeRotator` (.roll _returnvalue) (`local.InRot`) (.yaw _returnvalue))))
    (:`Z`
      (set `local.Rot` (`KismetMathLibrary.MakeRotator` (.roll _returnvalue) (.pitch _returnvalue) (`local.InRot`)))))
  (`SceneComponent.K2_SetWorldRotation` (`self.ProceduralMesh`) (`local.Rot`) false false))

(fn `UpdateArrow`
  (params (Length :type "Float (double-precision)"))
  (bind _arrow (`self.Arrow`))
  (`SceneComponent.K2_SetWorldLocation` _arrow (`KismetSystemLibrary.GetComponentBounds` (`self.ProceduralMesh`)) false false)
  (set `ArrowComponent.ArrowLength` (/ (`local.Length`) (`ArrowComponent.ArrowSize` (`self.Arrow`))) _arrow))

(fn `UpdateMesh`
  (params (Length :type "Float (double-precision)"))
  (locals (X :type Integer) (Y :type Integer) (Vertex :type "Array of Vector Structure"))
  (bind _vertexarr (`self.DrawQuad` Length))
  (`self.GenerateMesh` _vertexarr)
  (`self.UpdateArrow` (`local.Length`)))

(fn `UserConstructionScript`)